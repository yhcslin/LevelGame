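; BP_AppleSpawn is a spawner actor that keeps scattering apples across the play area, up to a cap.
; On BeginPlay it starts a looping half-second timer that calls Try Spawn Apple by name.
; That function counts live BP_Apple actors with GetAllActorsOfClass and, while under the cap, spawns one at a random XY point in a square around the world origin at fixed height.
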(event EventBeginPlay
  (Utilities|Time|SetTimerbyFunctionName 0 (Utilities|String|MakeLiteralString "Try Spawn Apple") 0.5 true))

(event Collision|EventActorBeginOverlap
  (params (OtherActor :type Actor%20Object%20Reference)))

(event EventTick
  (params (DeltaSeconds :type Float%20%28single-precision%29)))

(fn ConstructionScript)

(fn TrySpawnApple
  (bind _returnvalue (Math|Random|RandomPointinBoundingBox "0, 0, 0" "900.000000,900.000000,0.000000"))
  (bind _outactors (Actor|GetAllActorsOfClass "/Game/Blueprint/BP_Apple.BP_Apple_C"))
  (if (< (Utilities|Array|Length _outactors) 10)
    (bind _output_get (Variables|Default|SetRandLocation (Math|Vector|MakeVector (.x _returnvalue) (.y _returnvalue) (Math|Float|MakeLiteralFloat 2e+01))))
    (Game|SpawnActorfromClass "/Game/Blueprint/BP_Apple.BP_Apple_C" (Math|Transform|MakeTransform _output_get "0, 0, 0" "1.000000,1.000000,1.000000") "Undefined" "MultiplyWithRoot" 0 0)))