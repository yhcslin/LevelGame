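; BP_Apple is a collectible apple pickup that the player gathers toward a level-clear goal.
; When its Sphere overlaps BP_Player, it destroys itself and calls PickApple on the player.
; If the player's apple count then equals the hard-coded target of 20, it shows the UI_PassPA widget and enables the mouse cursor.
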(event OnComponentBeginOverlap(Sphere)
  (params (OverlappedComponent :type Primitive%20Component%20Object%20Reference) (OtherActor :type Actor%20Object%20Reference) (OtherComp :type Primitive%20Component%20Object%20Reference) (OtherBodyIndex :type Integer) (bFromSweep :type Boolean) (SweepResult :type Hit%20Result%20Structure%20%28by%20ref%29))
  (bind _asbp_player (Utilities|Casting|CastToBP_Player OtherActor))
  (Variables|Default|SetBP%20Player _asbp_player)
  (Actor|DestroyActor)
  (Default|PickApple (Variables|Default|GetBP%20Player))
  (if (== (Variables|/Game/Blueprint/BP_Player.BP_Player_C|GetAppleCnt (Variables|Default|GetBP%20Player)) 20)
    (bind _returnvalue (UserInterface|CreateWidget "/Game/Blueprint/UI/UI_PassPA.UI_PassPA_C"))
    (UserInterface|Viewport|AddtoViewport _returnvalue 0)
    (Variables|/Script/Engine.PlayerController|SetbShowMouseCursor (Game|GetPlayerController 0) true)))

(event EventBeginPlay)

(event Collision|EventActorBeginOverlap
  (params (OtherActor :type Actor%20Object%20Reference)))

(event EventTick
  (params (DeltaSeconds :type Float%20%28single-precision%29)))

(fn ConstructionScript)