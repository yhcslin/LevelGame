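; BP_RespawnPos is a one-shot checkpoint actor that sets the game's respawn position.
; When a BP_Player first overlaps its Capsule, it swaps the Plane's material to show activation and latches IsActivated.
; It then writes the Arrow component's world transform into the Transform variable on BP_LGGameMode, so the Arrow defines the stored location and facing.
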(event OnComponentBeginOverlap(Capsule)
  (params (OverlappedComponent :type Primitive%20Component%20Object%20Reference) (OtherActor :type Actor%20Object%20Reference) (OtherComp :type Primitive%20Component%20Object%20Reference) (OtherBodyIndex :type Integer) (bFromSweep :type Boolean) (SweepResult :type Hit%20Result%20Structure%20%28by%20ref%29))
  (if (not (Variables|Default|GetIsActivated))
    (Utilities|Casting|CastToBP_Player OtherActor)
    (Rendering|Material|SetMaterial (Variables|Default|GetPlane) 0 "/Engine/MapTemplates/Materials/BasicAsset01.BasicAsset01")
    (Variables|Default|SetIsActivated true)
    (bind _asbp_lggame_mode (Utilities|Casting|CastToBP_LGGameMode (Game|GetGameMode)))
    (Variables|/Game/Blueprints/BP_LGGameMode.BP_LGGameMode_C|SetTransform _asbp_lggame_mode (Transformation|GetWorldTransform (Variables|Default|GetArrow)))))

(event EventBeginPlay)

(event Collision|EventActorBeginOverlap
  (params (OtherActor :type Actor%20Object%20Reference)))

(event EventTick
  (params (DeltaSeconds :type Float%20%28single-precision%29)))

(fn ConstructionScript)