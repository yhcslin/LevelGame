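; Game mode Blueprint that handles player respawning and end-of-game score reset.
; RespawnCharacter spawns a new BP_Player at the Transform value and has player controller 0 possess it.
; EndGame sets Score on BP_LGGameInstance to zero, ignoring its IsWin input.
; EndPlay is empty, and a duplicate score reset in the event graph is never executed.
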(event EventEndPlay
  (params (EndPlayReason :type EEndPlayReason%20Enum :default "Destroyed")))

(fn ConstructionScript)

(fn RespawnCharacter
  (bind _returnvalue (Game|SpawnActorfromClass "/Game/Blueprints/BP_Player.BP_Player_C" (Variables|Default|GetTransform) "Undefined" "MultiplyWithRoot" 0 0))
  (Pawn|Possess (Game|GetPlayerController 0) _returnvalue))

(fn EndGame
  (params (bIsWin :type Boolean))
  (bind _asbp_lggame_instance (Utilities|Casting|CastToBP_LGGameInstance (Game|GetGameInstance)))
  (Variables|/Game/Blueprints/BP_LGGameInstance.BP_LGGameInstance_C|SetScore _asbp_lggame_instance 0))